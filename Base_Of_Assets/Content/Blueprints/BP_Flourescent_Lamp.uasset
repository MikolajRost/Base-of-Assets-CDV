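; BP_Flourescent_Lamp is an interactable fluorescent lamp that the player switches on and off.
; BeginInteraction runs a FlipFlop that shows or hides the RectLight and updates IsOn, with the first interaction always turning it on.
; Tick rewrites TextForInteractionPrompt every frame from IsOn to offer the matching "Press E" action.
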(event `self.ReceiveTick`
  (params (DeltaSeconds :type "Float (single-precision)"))
  (if (`self.IsOn?`)
    (set `self.TextForInteractionPrompt` "Press E to turn off")
    (else
      (set `self.TextForInteractionPrompt` "Press E to turn on"))))

(event `self.BeginInteraction`
  (bind _rectlight (`self.RectLight`))
  (`/Engine/EditorBlueprintResources/StandardMacros.FlipFlop`
    (:`A`
      (`SceneComponent.SetVisibility` _rectlight true false)
      (set `self.IsOn?` true))
    (:`B`
      (`SceneComponent.SetVisibility` _rectlight false false)
      (set `self.IsOn?` false))))

(fn `UserConstructionScript`
  (`parent.UserConstructionScript`))