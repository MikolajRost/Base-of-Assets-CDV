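; BP_CyberPunkRevolver is a revolver the player picks up and fires.
; BeginInteraction attaches its mesh to the first-person character's attachment point, disables mesh collision and flags the character as holding.
; UseItem activates Suction, waits briefly, then activates Gunshot and spawns a BP_Bullet at SpawnPoint.
; The forward AddForce on the bullet is disconnected, so this Blueprint applies no launch force.
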(event `self.BeginInteraction`
  (bind _staticmesh (`self.StaticMesh`))
  (bind _asbp_first_person_character (cast `/Game/FirstPerson/Blueprints/BP_FirstPersonCharacter` (`GameplayStatics.GetPlayerCharacter` 0)))
  (`SceneComponent.K2_AttachToComponent` _staticmesh (`/Game/FirstPerson/Blueprints/BP_FirstPersonCharacter.Attachment` _asbp_first_person_character) "None" "SnapToTarget" "SnapToTarget" "KeepWorld" true)
  (`PrimitiveComponent.SetCollisionEnabled` _staticmesh "NoCollision")
  (set `/Game/FirstPerson/Blueprints/BP_FirstPersonCharacter.IsHolding?` true _asbp_first_person_character))

(event `self.UseItem`
  (bind (_returnvalue_location _returnvalue_rotation) (`KismetMathLibrary.BreakTransform` (`SceneComponent.K2_GetComponentToWorld` (`self.SpawnPoint`))))
  (`ActorComponent.Activate` (`self.Suction`) false)
  (`KismetSystemLibrary.Delay` 0.2)
  (`|ExecutionSequence`
    (:`then_0`
      (`ActorComponent.Activate` (`self.Gunshot`) false))
    (:`then_1`
      (bind _returnvalue (`|SpawnActorFromClass` "/Game/Blueprints/BP_Bullet.BP_Bullet_C" (`KismetMathLibrary.MakeTransform` _returnvalue_location _returnvalue_rotation) "AlwaysSpawn" "MultiplyWithRoot" null null))
      (bind _asbp_first_person_character (cast `/Game/FirstPerson/Blueprints/BP_FirstPersonCharacter` (`GameplayStatics.GetPlayerCharacter` 0))))))

(fn `UserConstructionScript`
  (`parent.UserConstructionScript`))