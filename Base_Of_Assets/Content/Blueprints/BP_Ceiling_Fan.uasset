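; An interactable ceiling fan that the player switches on and off.
; BeginInteraction alternates through a FlipFlop, setting IsON and either playing or stopping the RotateFan timeline.
; While playing, the timeline's Rotate track drives the relative yaw of the fan mesh.
; Tick rewrites the interaction prompt every frame to offer turning the fan on or off according to IsON.
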(event `self.ReceiveTick`
  (params (DeltaSeconds :type "Float (single-precision)"))
  (if (`self.Is ON?`)
    (set `self.TextForInteractionPrompt` "Press E to turn off")
    (else
      (set `self.TextForInteractionPrompt` "Press E to turn on"))))

(event `self.BeginInteraction`
  (`/Engine/EditorBlueprintResources/StandardMacros.FlipFlop`
    (:`A`
      (set `self.Is ON?` true)
      (bind (_direction _rotate) (`Timeline|Rotate Fan` :!label _label)
        (:`Update`
          (`SceneComponent.K2_SetRelativeRotation` (`self.SM_Ceilingfan_01_object_002_low`) (`KismetMathLibrary.MakeRotator` 0.0 0.0 _rotate) false false))))
    (:`B`
      (set `self.Is ON?` false)
      (goto _label :!via `Stop`))))

(fn `UserConstructionScript`
  (`parent.UserConstructionScript`))