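; BP_Interactable is an interactable actor that signals interaction with a highlight and an on-screen prompt.
; Its open event applies a highlight overlay material to the static mesh and creates a UW_Prompt widget with configurable text; its close event removes both.
; BeginInteraction and UseItem clear CanInteract and CanUse respectively when the SingleInteraction or SingleUse flag is set.
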(event `Open Highlight & Prompt`
  (`MeshComponent.SetOverlayMaterial` (`self.StaticMesh`) "/Game/Materials/M_Highlight.M_Highlight")
  (bind _returnvalue (`|CreateWidget` "/Game/UI/UW_Prompt.UW_Prompt_C" (`GameplayStatics.GetPlayerController` 0)))
  (bind _output_get (set `self.PromptRef` _returnvalue))
  (`UserWidget.AddToViewport` _output_get 0)
  (`TextBlock.SetText` (`/Game/UI/UW_Prompt.Prompt` (`self.PromptRef`)) (`self.TextForInteractionPrompt`)))

(event `Close Highlight & Prompt`
  (`MeshComponent.SetOverlayMaterial` (`self.StaticMesh`) null)
  (`Widget.RemoveFromParent` (`self.PromptRef`)))

(event `BeginInteraction`
  (if (`self.SingleInteraction?`)
    (set `self.CanInteract?` false)))

(event `UseItem`
  (if (`self.SingleUse?`)
    (set `self.CanUse?` false)))

(fn `UserConstructionScript`)